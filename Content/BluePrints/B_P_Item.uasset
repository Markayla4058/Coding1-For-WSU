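; B_P_Item is an item Blueprint with a name, elemental type and damage value, apparently prototyping elemental weakness damage.
; Construction replaces a default "Item" name by a random pick from an array holding only one connected name.
; GetDamage doubles damage when the victim's element, offset modulo four, matches the item's, returning doubled and normal results on separate outputs.
; BeginPlay debug-prints the name, element and doubled-damage output against a hardcoded element.
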(event EventBeginPlay
  (Development|PrintString (Variables|Default|GetName))
  (bind _damage (CallFunction|GetDamage "NewEnumerator3"))
  (Development|PrintString (Utilities|String|Append "Our elemtn type is earth." (Utilities|String|EnumtoString (Variables|Default|GetElementalType)) "" (Utilities|String|ToString(Integer) _damage))))

(event Collision|EventActorBeginOverlap
  (params (OtherActor :type Actor%20Object%20Reference)))

(event EventTick
  (params (DeltaSeconds :type Float%20%28single-precision%29)))

(fn ConstructionScript
  (bind _returnvalue (Utilities|String|MakeLiteralString "Fay"))
  (bind _array (Utilities|Array|MakeArray _returnvalue))
  (if (Utilities|Enum|Equal(Enum) (Variables|Default|GetName) "Item")
    (Utilities|Array|Shuffle _array)
    (Variables|Default|SetName (Utilities|Array|Get(acopy) _array (Math|Random|RandomIntegerinRange 0 (Utilities|Array|Length _array))))
    (Development|PrintString (Utilities|String|Append "" ""))))

(fn Constructor)

(fn GetDamage
  (params (Victum :type ElementalType%20Enum :default "NewEnumerator0"))
  (LocalVariables|SetReturnedDamage (Variables|Default|GetDamage))
  (if (== (Math|Integer|%(Integer) (+ (Math|Conversions|ToInteger(Byte) Victum) 2) 4) (Math|Conversions|ToInteger(Byte) (Variables|Default|GetElementalType)))
    (bind _output_get (LocalVariables|SetReturnedDamage (* (Variables|Default|GetDamage) 2)))
    (return _output_get 0)
    (else
      (return 0 (LocalVariables|GetReturnedDamage)))))
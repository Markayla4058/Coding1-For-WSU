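; BP_CoolBox_Auto5 is a box actor that spawns a Key_BP actor every second for as long as it runs.
; BeginPlay zeroes KeySpawnLocation and prints debug messages with the actor's name, the Cube's world location and that location plus the offset.
; A looping Delay then repeats the spawn, using KeySpawnLocation directly as a world position, so keys appear at the origin rather than at the Cube.
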(event EventBeginPlay
  (bind _cube (Variables|Default|GetCube))
  (bind _returnvalue (Transformation|GetWorldLocation _cube))
  (bind _output_get (Variables|Default|SetKeySpawnLocation "0, 0, 0"))
  (Development|PrintString (Utilities|String|Append (Utilities|GetDisplayName self) "exists!") true true "(R=0.000000,G=0.660000,B=1.000000,A=1.000000)" 1e+01)
  (Development|PrintString (Utilities|String|ToString(Vector) _returnvalue) true true "(R=0.003284,G=0.600000,B=0.000000,A=1.000000)" 1e+01)
  (Development|PrintString (Utilities|String|ToString(Vector) (+ _returnvalue _output_get)) true true "(R=1.000000,G=0.024000,B=0.841116,A=1.000000)" 1e+01)
  (Game|SpawnActorfromClass "/Game/ThirdPerson/Maps/BluePrint/Key_BP.Key_BP_C" (Math|Transform|MakeTransform _output_get "0, 0, 0" "1.000000,1.000000,1.000000") "Undefined" "MultiplyWithRoot" 0 0 :!label _label)
  (Utilities|FlowControl|Delay 1.0)
  (goto _label))

(event Collision|EventActorBeginOverlap
  (params (OtherActor :type Actor%20Object%20Reference)))

(event EventTick
  (params (DeltaSeconds :type Float%20%28single-precision%29)))

(fn ConstructionScript)